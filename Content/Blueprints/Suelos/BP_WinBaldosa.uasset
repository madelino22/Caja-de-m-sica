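; BP_WinBaldosa is a Sokoban goal tile that detects music boxes (BP_CajaMusica) landing on it.
; Box overlaps check the box's instrument against the tile's, with one enum value acting as a wildcard for any instrument.
; A match plays the box's track, notifies the BP_SokobanLogic game mode and, if BlockCajaMusica is set, disables pushing.
; When a matching box leaves, its track stops and the game mode is notified.
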(event `self.ReceiveBeginPlay`
  (`parent.ReceiveBeginPlay`))

(event `self.Box.OnComponentBeginOverlap`
  (params (OverlappedComponent :type "PrimitiveComponent Object Reference") (OtherActor :type "Actor Object Reference") (OtherComp :type "PrimitiveComponent Object Reference") (OtherBodyIndex :type Integer) (bFromSweep :type Boolean) (SweepResult :type "HitResult Structure (by ref)"))
  (bind _asbp_caja_musica (cast `/Game/Blueprints/BP_CajaMusica` OtherActor))
  (bind _compatible (`self.checkBoxBaldosaComptible` (`/Game/Blueprints/BP_CajaMusica.MyInstrument` _asbp_caja_musica)))
  (if _compatible
    (`|ExecutionSequence`
      (:`then_0`
        ;[1 1 1] Cambiar volumen del track cuando la caja esté bien colocada
        (`/Game/Blueprints/BP_CajaMusica.playTrack` _asbp_caja_musica))
      (:`then_1`
        ;[1 1 1] entonces cuéntala en el sokoban logic
        (bind _asbp_sokoban_logic (cast `/Game/Blueprints/BP_SokobanLogic` (`GameplayStatics.GetGameMode`)))
        (`/Game/Blueprints/BP_SokobanLogic.OnBoxLanded` _asbp_sokoban_logic))
      (:`then_2`
        ;[1 1 1] bloque la caja si flag esta a true
        (if (`self.BlockCajaMusica`)
          (`/Game/Blueprints/Components/BPC_Pushable.Disable Push` (`/Game/Blueprints/BP_MuroMovible.BPC_Pushable` _asbp_caja_musica)))))))

(event `self.Box.OnComponentEndOverlap`
  (params (OverlappedComponent :type "PrimitiveComponent Object Reference") (OtherActor :type "Actor Object Reference") (OtherComp :type "PrimitiveComponent Object Reference") (OtherBodyIndex :type Integer))
  (bind _asbp_caja_musica (cast `/Game/Blueprints/BP_CajaMusica` OtherActor))
  (bind _compatible (`self.checkBoxBaldosaComptible` (`/Game/Blueprints/BP_CajaMusica.MyInstrument` _asbp_caja_musica)))
  (if _compatible
    (`|ExecutionSequence`
      (:`then_0`
        (`/Game/Blueprints/BP_CajaMusica.stopTrack` _asbp_caja_musica))
      (:`then_1`
        (bind _asbp_sokoban_logic (cast `/Game/Blueprints/BP_SokobanLogic` (`GameplayStatics.GetGameMode`)))
        (`/Game/Blueprints/BP_SokobanLogic.OnBoxUnlanded` _asbp_sokoban_logic)))))

(fn `checkBoxBaldosaComptible`
  (params (boxInstrumentTag :type "/Game/Blueprints/E_MyInstruments Enum" :default "NewEnumerator0"))
  (returns (compatible :type Boolean))
  (return (or (`|EnumEquality` (`self.MyInstrument`) "NewEnumerator3") (`|EnumEquality` (`self.MyInstrument`) boxInstrumentTag))))

(fn `UserConstructionScript`
  (`parent.UserConstructionScript`))