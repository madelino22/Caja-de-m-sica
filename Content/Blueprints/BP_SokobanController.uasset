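; Player controller for a Sokoban puzzle game that turns Enhanced Input actions into grid moves, undo and level restart.
; On BeginPlay it caches the Sokoban player pawn, shows the main HUD, prepares a reset widget and adds the input mapping context.
; Direction inputs ask the pawn to step 100 units and rotate it to face that way.
; Restart is held, filling a progress bar before reloading the current level.
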(event `self.ReceiveBeginPlay`
  (`|ExecutionSequence`
    (:`then_0`
      (bind _asbp_sokoban_player (cast `/Game/Blueprints/BP_SokobanPlayer` (`GameplayStatics.GetPlayerPawn` 0)))
      (set `self.Sokoban Player` _asbp_sokoban_player))
    (:`then_1`
      (bind _returnvalue (`|CreateWidget` "/Game/HUD/MainHUD.MainHUD_C"))
      (`UserWidget.AddToViewport` _returnvalue 0)
      (bind _returnvalue_2 (`|CreateWidget` "/Game/HUD/Reseteo.Reseteo_C"))
      (set `self.HUD reset` _returnvalue_2))
    (:`then_2`
      (`EnhancedInputSubsystemInterface.AddMappingContext` (subsystem `EnhancedInputLocalPlayerSubsystem`) "/Game/Inputs/IMC_Context.IMC_Context" 0 (struct)))))

(event `EnhancedInput|/Game/Inputs/IA_LeftMovement`
  (params (ActionValue :type Boolean) (ElapsedSeconds :type "Float (double-precision)") (TriggeredSeconds :type "Float (double-precision)") (InputAction :type "InputAction Object Reference" :default "/Game/Inputs/IA_LeftMovement.IA_LeftMovement"))
  (bind _sokoban_player (`self.Sokoban Player`))
  (:`Triggered`
    (`/Game/Blueprints/BP_SokobanPlayer.Try Move Towards` _sokoban_player (0.0 -100.0 0.0))
    (`self.K2_SetActorRotation` _sokoban_player (struct :`Yaw` -90.0) false)))

(event `EnhancedInput|/Game/Inputs/IA_UpMovement`
  (params (ActionValue :type Boolean) (ElapsedSeconds :type "Float (double-precision)") (TriggeredSeconds :type "Float (double-precision)") (InputAction :type "InputAction Object Reference" :default "/Game/Inputs/IA_UpMovement.IA_UpMovement"))
  (bind _sokoban_player (`self.Sokoban Player`))
  (:`Triggered`
    (`/Game/Blueprints/BP_SokobanPlayer.Try Move Towards` _sokoban_player (100.0 0.0 0.0))
    (`self.K2_SetActorRotation` :`self` _sokoban_player)))

(event `EnhancedInput|/Game/Inputs/IA_DownMovement`
  (params (ActionValue :type Boolean) (ElapsedSeconds :type "Float (double-precision)") (TriggeredSeconds :type "Float (double-precision)") (InputAction :type "InputAction Object Reference" :default "/Game/Inputs/IA_DownMovement.IA_DownMovement"))
  (bind _sokoban_player (`self.Sokoban Player`))
  (:`Triggered`
    (`/Game/Blueprints/BP_SokobanPlayer.Try Move Towards` _sokoban_player (-100.0 0.0 0.0))
    (`self.K2_SetActorRotation` _sokoban_player (struct :`Yaw` 180.0) false)))

(event `EnhancedInput|/Game/Inputs/IA_RightMovement`
  (params (ActionValue :type Boolean) (ElapsedSeconds :type "Float (double-precision)") (TriggeredSeconds :type "Float (double-precision)") (InputAction :type "InputAction Object Reference" :default "/Game/Inputs/IA_RightMovement.IA_RightMovement"))
  (bind _sokoban_player (`self.Sokoban Player`))
  (:`Triggered`
    (`/Game/Blueprints/BP_SokobanPlayer.Try Move Towards` _sokoban_player (0.0 100.0 0.0))
    (`self.K2_SetActorRotation` _sokoban_player (struct :`Yaw` 90.0) false)))

(event `EnhancedInput|/Game/Inputs/IA_Undo`
  (params (ActionValue :type Boolean) (ElapsedSeconds :type "Float (double-precision)") (TriggeredSeconds :type "Float (double-precision)") (InputAction :type "InputAction Object Reference" :default "/Game/Inputs/IA_Undo.IA_Undo"))
  (:`Triggered`
    (`/Game/Blueprints/BP_SokobanPlayer.ControlZ` (`self.Sokoban Player`))))

(event `EnhancedInput|/Game/Inputs/IA_RestartLevel`
  (params (ActionValue :type Boolean) (ElapsedSeconds :type "Float (double-precision)") (TriggeredSeconds :type "Float (double-precision)") (InputAction :type "InputAction Object Reference" :default "/Game/Inputs/IA_RestartLevel.IA_RestartLevel"))
  (bind _hud_reset (`self.HUD reset`))
  (bind _barraprogreso (`/Game/HUD/Reseteo.BarraProgreso` _hud_reset))
  (:`Triggered`
    (bind _returnvalue (`GameplayStatics.GetCurrentLevelName` true))
    (`GameplayStatics.OpenLevel` (`KismetStringLibrary.Conv_StringToName` _returnvalue)))
  (:`Started`
    (`UserWidget.AddToViewport` _hud_reset 0)
    (`ProgressBar.SetPercent` _barraprogreso 0.0))
  (:`Ongoing`
    (`ProgressBar.SetPercent` _barraprogreso (/ ElapsedSeconds 2.0)))
  (:`Canceled`
    (`Widget.RemoveFromParent` _hud_reset :!label _label))
  (:`Completed`
    (goto _label)))

(fn `UserConstructionScript`)