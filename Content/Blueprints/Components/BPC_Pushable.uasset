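; BPC_Pushable is an actor component that lets its owner be pushed by a displacement when pushing is enabled and the applied force meets its required threshold.
; Push line-traces from just above the owner's origin along the displacement to find obstacles.
; A pushable obstacle is pushed recursively with the leftover force, enabling chained pushes.
; The owner moves without sweep only if the path clears, otherwise Push reports failure.
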(fn `Disable Push`
  (set `self.Push enabled` false))

(fn `Enable Push`
  (set `self.Push enabled` true))

(fn `Push`
  (params (Despl :type "Vector Structure") (Fuerza :type Integer))
  (returns (Pushed :type Boolean) (Obstacle :type "Actor Object Reference"))
  (bind _returnvalue (`self.GetOwner`))
  (bind _returnvalue_2 (+ (`Actor.K2_GetActorLocation` _returnvalue) (0.0 0.0 50.0)))
  (if (`self.Push enabled`)
    (if (>= Fuerza (`self.Fuerza Necesaria`))
      (bind (_outhit _returnvalue_3) (`KismetSystemLibrary.LineTraceSingle` _returnvalue_2 (+ _returnvalue_2 Despl) "TraceTypeQuery1"))
      (if _returnvalue_3
        (bind _returnvalue_4 (`Actor.GetComponentByClass` (`.HitActor` (`GameplayStatics.BreakHitResult` _outhit)) "BPC_Pushable_C"))
        (`/Engine/EditorBlueprintResources/StandardMacros.IsValid` _returnvalue_4
          (:`Is Valid`
            (bind (_pushed _obstacle) (`self.Push` _returnvalue_4 (`local.Despl`) (- (`local.Fuerza`) (`self.Fuerza Necesaria`))))
            (if _pushed
              _
              (else
                (return false _obstacle))))
          (:`Is Not Valid`
            (return false (`.HitActor` (`GameplayStatics.BreakHitResult` _outhit))))))
      (`Actor.K2_AddActorWorldOffset` _returnvalue Despl false false)
      (return true (`.HitActor` (`GameplayStatics.BreakHitResult` _outhit)))
      (else
        _)))
  (return false null))