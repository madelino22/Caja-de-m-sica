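; Sokoban puzzle logic Blueprint that counts moves and detects when every music box in the level is placed.
; Binds to the player's move callback to increment a local counter and the TotalMovements counter in the BP_SokobanData game instance.
; Counts BP_CajaMusica actors one tick after BeginPlay, tracks landed and unlanded events, and disables pushing on all music boxes once the placed count matches the total.
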(event `Player moved`
  ;[1 1 1] Gestión número de pasos
  (`/Engine/EditorBlueprintResources/StandardMacros.IncrementInt` (`self.Num movements`)
    (:`  `
      (bind _asbp_sokoban_data (cast `/Game/Blueprints/BP_SokobanData` (`GameplayStatics.GetGameInstance`)))
      (`/Engine/EditorBlueprintResources/StandardMacros.IncrementInt` (`/Game/Blueprints/BP_SokobanData.Total movements` _asbp_sokoban_data)))))

(event `self.ReceiveBeginPlay`
  (`|ExecutionSequence`
    (:`then_0`
      ;[1 1 1] Gestión número de pasos
      (bind _asbp_sokoban_player (cast `/Game/Blueprints/BP_SokobanPlayer` (`GameplayStatics.GetPlayerPawn` 0)))
      (add `/Game/Blueprints/BP_SokobanPlayer.PlayerMoved` _asbp_sokoban_player (delegate `Player moved`)))
    (:`then_1`
      ;[1 1 1] Set número de cajas totales en este nivel
      (`KismetSystemLibrary.DelayUntilNextTick`)
      (bind _outactors (`GameplayStatics.GetAllActorsOfClass` "/Game/Blueprints/BP_CajaMusica.BP_CajaMusica_C"))
      (set `self.nCajasMusicaTotales` (`KismetArrayLibrary.Array_Length` _outactors)))))

(event `OnBoxLanded`
  (`/Engine/EditorBlueprintResources/StandardMacros.IncrementInt` (`self.nCajasMusicaColocadas`)
    (:`  `
      ;[1 1 1] Si nivel es resuelto, bloquea todos los muros movibles
      (if (== (`self.nCajasMusicaColocadas`) (`self.nCajasMusicaTotales`))
        (bind _outactors (`GameplayStatics.GetAllActorsOfClass` "/Game/Blueprints/BP_CajaMusica.BP_CajaMusica_C"))
        (for _array_element _outactors
          (`/Game/Blueprints/Components/BPC_Pushable.Disable Push` (`/Game/Blueprints/BP_MuroMovible.BPC_Pushable` _array_element)))))))

(event `OnBoxUnlanded`
  (`/Engine/EditorBlueprintResources/StandardMacros.DecrementInt` (`self.nCajasMusicaColocadas`)))

(fn `UserConstructionScript`)