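; Player pawn for a Sokoban-style box-pushing game, with movement, undo and a pause menu.
; TryMoveTowards pushes through the pushable component; successful moves are recorded with any moved BP_MuroMovible and announced, while failures send a bump message to the obstacle.
; ControlZ pops that MovData stack, built with array-backed push/pop macros, and shifts player and box back by the inverse displacement.
; The pause input opens PauseMenu, shows the cursor and pauses the game.
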(event `self.ReceiveBeginPlay`
  (bind _returnvalue (`GameplayStatics.GetPlayerController` 0))
  (set `PlayerController.bShowMouseCursor` false _returnvalue)
  (`WidgetBlueprintLibrary.SetInputMode_GameOnly` _returnvalue))

(event `EnhancedInput|/Game/Inputs/IA_Pause`
  (params (ActionValue :type Boolean) (ElapsedSeconds :type "Float (double-precision)") (TriggeredSeconds :type "Float (double-precision)") (InputAction :type "InputAction Object Reference" :default "/Game/Inputs/IA_Pause.IA_Pause"))
  (bind _returnvalue (`GameplayStatics.GetPlayerController` 0))
  ;[1 1 1] pausar el juego con la P, y mostrar el cursor
  (:`Started`
    (bind _returnvalue_2 (`|CreateWidget` "/Game/UI/PauseMenu.PauseMenu_C"))
    (`UserWidget.AddToViewport` _returnvalue_2 0)
    (set `PlayerController.bShowMouseCursor` true _returnvalue)
    (`WidgetBlueprintLibrary.SetInputMode_UIOnlyEx` _returnvalue null)
    (`GameplayStatics.SetGamePaused` true)))

(fn `ControlZ`
  (bind _movsdata (`self.MovsData`))
  (bind _returnvalue (`KismetArrayLibrary.Array_IsEmpty` _movsdata))
  (`KismetSystemLibrary.PrintString` (`KismetStringLibrary.Conv_BoolToString` _returnvalue))
  (if _returnvalue
    (return)
    (else
      (bind _mov_data (`self.STACK_POP` _movsdata)
        (:`Exit`
          (bind _returnvalue_2 (* (break `/Game/Blueprints/MovData` _mov_data) (-1.0 -1.0 -1.0)))
          (`self.K2_SetActorLocation` (+ _returnvalue_2 (`self.K2_GetActorLocation`)))
          (if (`KismetSystemLibrary.IsValid` (`.Caja_6_C8AF70284D0A75E14ECBE2943F7862F9` (break `/Game/Blueprints/MovData` _mov_data)))
            (`self.K2_SetActorLocation` (`.Caja_6_C8AF70284D0A75E14ECBE2943F7862F9` (break `/Game/Blueprints/MovData` _mov_data)) (+ (`self.K2_GetActorLocation` (`.Caja_6_C8AF70284D0A75E14ECBE2943F7862F9` (break `/Game/Blueprints/MovData` _mov_data))) _returnvalue_2) false false)
            (return)))))))

(fn `PrintMovsData`
  (locals (NewLocalVar :type "Array of /Game/Blueprints/MovData Structure"))
  (bind _movsdata (`self.MovsData`))
  (for _array_element _movsdata
    (`KismetSystemLibrary.PrintString` (`KismetTextLibrary.Conv_TextToString` (`|FormatText` "{Vector}{Bool}{int}" (`KismetStringLibrary.Conv_VectorToString` (break `/Game/Blueprints/MovData` _array_element)) (`KismetSystemLibrary.IsValid` (`.Caja_6_C8AF70284D0A75E14ECBE2943F7862F9` (break `/Game/Blueprints/MovData` _array_element))) (`KismetArrayLibrary.Array_Length` _movsdata))) true true (struct :`G` 0.66 :`B` 1.0 :`A` 1.0) 15.0)))

(fn `Save Movement`
  (params (despl :type "Vector Structure") (muroMov :type "/Game/Blueprints/BP_MuroMovible Object Reference"))
  (bind _index (`self.STACK_PUSH` (`self.MovsData`) (make `/Game/Blueprints/MovData` despl muroMov))
    (:`Exit`
      (if (>= _index 5)
        _))))

(fn `Try Move Towards`
  (params (Despl :type "Vector Structure"))
  (returns (Success :type Boolean))
  (bind (_pushed _obstacle) (`/Game/Blueprints/Components/BPC_Pushable.Push` (`self.BPC_Pushable`) Despl (`self.Fuerza`)))
  (if _pushed
    (bind _asbp_muro_movible (cast `/Game/Blueprints/BP_MuroMovible` _obstacle)
      (:`then`
        (`self.Save Movement` Despl _asbp_muro_movible))
      (:`CastFailed`
        (`self.Save Movement` Despl)))
    (`self.PlayerMoved`)
    (return true)
    (else
      (`self.TryBump` _obstacle)
      (return false))))

(fn `TryBump`
  (params (Object :type "Actor Object Reference"))
  (message `/Game/Blueprints/BPI_Chocable.Something Bump` Object (0.0 0.0 0.0)))

(fn `UserConstructionScript`)