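; BP_SokobanCamera is a Sokoban camera with spring-follow and occlusion-avoidance logic, currently disconnected from its events, as is a MapBuilder-based placement call.
; ChangeTargetActor stores offset and distance; UpdateRotation eases toward the target's eye height.
; UpdatePosition line-traces samples between natural and last-resort positions, easing toward the first clear one.
; Blockers implementing BPI_AmableConCamara are notified and count as clear, though both position helpers leave their computations unused.
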(event `self.ReceiveBeginPlay`)

(event `self.ReceiveTick`
  (params (DeltaSeconds :type "Float (single-precision)")))

(fn `Can See Target From`
  (params (Location :type "Vector Structure"))
  (returns (`is visible` :type Boolean))
  (bind (_outhit _returnvalue) (`KismetSystemLibrary.LineTraceSingle` Location (`self.Get Look At Position`) "TraceTypeQuery1" false (`|MakeArray` (`self.Target`))))
  (if _returnvalue
    (if (`KismetSystemLibrary.DoesImplementInterface` (`.HitActor` (`GameplayStatics.BreakHitResult` _outhit)) "/Game/Blueprints/BPI_AmableConCamara.BPI_AmableConCamara_C")
      (message `/Game/Blueprints/BPI_AmableConCamara.OnEstasEnMedio` (`.HitActor` (`GameplayStatics.BreakHitResult` _outhit)))
      (return true)
      (else
        (return false)))
    (else
      (return true))))

(fn `Change Target Actor`
  (params (`New target` :type "Actor Object Reference"))
  (bind _returnvalue (- (`self.K2_GetActorLocation`) (`self.Get Look At Position`)))
  (bind _output_get (set `self.Target` `New target`))
  (`/Engine/EditorBlueprintResources/StandardMacros.IsValid` _output_get
    (:`Is Valid`
      (set `self.TargetOffset` _returnvalue)
      (set `self.TargetDistance` (`KismetMathLibrary.VSize` _returnvalue)))))

(fn `Get Look At Position`
  (returns (Position :type "Vector Structure"))
  (return (+ (`self.K2_GetActorLocation` (`self.Target`)) (`KismetMathLibrary.MakeVector` 0.0 0.0 (`self.Target Eyes Height`)))))

(fn `Update Position`
  (locals (`Selected position` :type "Vector Structure"))
  (`|ExecutionSequence`
    (:`then_0`
      (set `local.Selected position` (`self.Get Last Resort Position`))
      (for _index (range 11)
        (bind _returnvalue (`KismetMathLibrary.VLerp` (`self.Get Natural Position`) (`self.Get Last Resort Position`) (`KismetMathLibrary.NormalizeToRange` (`KismetMathLibrary.Conv_IntToDouble` _index) 0.0 10.0)))
        (bind _is_visible (`self.Can See Target From` _returnvalue))
        (if _is_visible
          (set `local.Selected position` _returnvalue)
          (break))))
    (:`then_1`
      (`self.K2_SetActorLocation` (`KismetMathLibrary.VLerp` (`self.K2_GetActorLocation`) (`local.Selected position`) (* (`self.Spring factor`) (`GameplayStatics.GetWorldDeltaSeconds`)))))))

(fn `Update Rotation`
  (`SceneComponent.K2_SetWorldRotation` (`self.SceneComponent`) (`KismetMathLibrary.RLerp` (`self.K2_GetActorRotation`) (`KismetMathLibrary.FindLookAtRotation` (`self.K2_GetActorLocation`) (`self.Get Look At Position`)) (* (`self.Rotation spring factor`) (`GameplayStatics.GetWorldDeltaSeconds`))) false false))

(fn `UserConstructionScript`)