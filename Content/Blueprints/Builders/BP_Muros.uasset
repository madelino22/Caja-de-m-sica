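; BP_Muros is a builder actor that lays out a tile grid of walls from the Description array of strings.
; Its construction script maps each string index to X and character index to Y on a 100-unit grid, adding a child actor component per recognized character.
; CodeToClass turns "W" into BP_Muro and skips other characters; a BP_CajaMusica return exists but is never reached.
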(fn `Code to class`
  (params (StringCode :type String))
  (returns (TileClass :type "Actor Class Reference"))
  (switch `string` StringCode
    (:`Default`
      (return null))
    (:`W`
      (return "/Game/Blueprints/BP_Muro.BP_Muro_C"))))

(fn `Create Object`
  (params (TileX :type Integer) (TileY :type Integer) (`Tile Class` :type "Actor Class Reference"))
  (if (`KismetSystemLibrary.IsValidClass` `Tile Class`)
    (bind _returnvalue (`AddComponent|NODE_AddChildActorComponent-0` :`RelativeTransform` (`KismetMathLibrary.Conv_VectorToTransform` (`KismetMathLibrary.MakeVector` (`KismetMathLibrary.Conv_IntToDouble` (* (`local.TileX`) 100)) (`KismetMathLibrary.Conv_IntToDouble` (* (`local.TileY`) 100))))))
    (`ChildActorComponent.SetChildActorClass` _returnvalue (`local.Tile Class`))))

(fn `UserConstructionScript`
  (locals (NumCadena :type Integer) (NumChar :type Integer))
  ;[1 1 1] para cada cadena
  (for (_array_element _array_index) (`self.Description`)
    (set `local.NumCadena` _array_index)
    ;;[1 1 1] Para cada caracter
    (for (_array_element_2 _array_index_2) (`KismetStringLibrary.GetCharacterArrayFromString` _array_element)
      (set `local.NumChar` _array_index_2)
      ;;;[1 1 1] Creamos el objecto
      (bind _tileclass (`self.Code to class` _array_element_2))
      (`self.Create Object` (`local.NumCadena`) (`local.NumChar`) _tileclass))))