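; BP_Rectangle is a builder actor that lays out a hollow rectangular border of blocks, sized in tiles by TamX and TamY.
; The construction script runs two edge loops, the second skipping the corners, and CreateObject adds each BlockEntity as a child actor component on a 100-unit grid.
; SetCameraPos returns a camera position from the actor location plus half the rectangle size, at a fixed height.
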(fn `Create object`
  (params (`Tile X` :type Integer) (`Tile Y` :type Integer))
  (bind _returnvalue (`AddComponent|NODE_AddChildActorComponent-0` :`RelativeTransform` (`KismetMathLibrary.Conv_VectorToTransform` (`KismetMathLibrary.MakeVector` (`KismetMathLibrary.Conv_IntToDouble` (* (`local.Tile X`) 100)) (`KismetMathLibrary.Conv_IntToDouble` (* (`local.Tile Y`) 100))))))
  (`ChildActorComponent.SetChildActorClass` _returnvalue (`self.Block entity`)))

(fn `SetCameraPos`
  (returns (DesiredPos :type "Vector Structure"))
  (locals (LastObjectPos :type "Vector Structure"))
  (bind _returnvalue (`self.K2_GetActorLocation`))
  (bind (_returnvalue_x _returnvalue_y) (`KismetMathLibrary.BreakVector` (/ (+ (`KismetMathLibrary.MakeVector` (`KismetMathLibrary.Conv_IntToDouble` (* (`self.Tam X`) 100)) (`KismetMathLibrary.Conv_IntToDouble` (* (`self.Tam Y`) 100))) _returnvalue _returnvalue) 2)))
  (return (`KismetMathLibrary.MakeVector` _returnvalue_x _returnvalue_y 900.0)))

(fn `UserConstructionScript`
  (`|ExecutionSequence`
    (:`then_0`
      ;[1 1 1] Verticales (misma Y)
      (for _index (range (`self.Tam X`))
        (`self.Create object` _index)
        (`self.Create object` _index (- (`self.Tam Y`) 1))))
    (:`then_1`
      ;[1 1 1] Horizontales (misma X)
      (for _index_2 (range 1 (+ (- (`self.Tam Y`) 2) 1))
        (`self.Create object` 0 _index_2)
        (`self.Create object` (- (`self.Tam X`) 1) _index_2)))))