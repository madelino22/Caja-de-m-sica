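; BP_MusicVolume is a trigger volume that switches the music when a BP_MuroMovible actor enters it.
; At BeginPlay it caches the first BP_MusicManager found in the level.
; When its CajaColocada component begins overlap, it casts the other actor to BP_MuroMovible, checks that it is not CajaColocada itself, and passes MusicToPlayOnOverlap to the manager's ChangeMusicTo.
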(event `self.ReceiveBeginPlay`
  (bind _outactors (`GameplayStatics.GetAllActorsOfClass` "/Game/Blueprints/Sound/BP_MusicManager.BP_MusicManager_C"))
  (set `self.MusicManagerRef` (`|GetArrayItem` _outactors)))

(event `self.CajaColocada.OnComponentBeginOverlap`
  (params (OverlappedComponent :type "PrimitiveComponent Object Reference") (OtherActor :type "Actor Object Reference") (OtherComp :type "PrimitiveComponent Object Reference") (OtherBodyIndex :type Integer) (bFromSweep :type Boolean) (SweepResult :type "HitResult Structure (by ref)"))
  (bind _asbp_muro_movible (cast `/Game/Blueprints/BP_MuroMovible` OtherActor))
  (if (not (== (`self.CajaColocada`) _asbp_muro_movible))
    (`/Game/Blueprints/Sound/BP_MusicManager.ChangeMusicTo` (`self.MusicManagerRef`) (`self.MusicToPlayOnOverlap`))))

(fn `UserConstructionScript`)