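; BP_Columna is a column actor that temporarily changes material when told it is in the way through OnEstasEnMedio.
; The event applies MaterialEstorbando, and a short retriggerable delay restores MaterialNormal once the calls stop arriving.
; CambiaMaterial sets the first material slot on every static mesh component, and the construction script uses it to apply the normal material initially.
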(event `/Game/Blueprints/BPI_AmableConCamara.OnEstasEnMedio`
  (`self.CambiaMaterial` (`self.MaterialEstorbando`))
  (`KismetSystemLibrary.RetriggerableDelay` 0.2)
  (`self.CambiaMaterial` (`self.MaterialNormal`)))

(fn `CambiaMaterial`
  (params (NewMaterial :type "Material Object Reference"))
  (for _array_element (`self.K2_GetComponentsByClass` "/Script/Engine.StaticMeshComponent")
    (`PrimitiveComponent.SetMaterial` _array_element 0 NewMaterial)))

(fn `UserConstructionScript`
  (`self.CambiaMaterial` (`self.MaterialNormal`)))