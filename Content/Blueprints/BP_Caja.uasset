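; BP_Caja is a box actor with an optional scale animation and a toggleable pushable behavior.
; On BeginPlay, if ActivarAnimacion is set, the Bailongo timeline plays or reverses according to Modo, driving the actor's 3D scale per axis.
; The timeline's play rate is the inverse of TiempoAnimacion, so that variable controls animation duration.
; SetIsPushable enables or disables pushing through the Pushable component.
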(event `self.ReceiveBeginPlay`
  (if (`self.Activar Animacion`)
    (`TimelineComponent.SetPlayRate` (`self.Bailongo`) (/ 1.0 (`self.Tiempo Animacion`)))
    (if (`self.Modo`)
      (bind (_direction _x_pos _y_pos _z_pos) (`Timeline|Bailongo` :!label _label)
        (:`Update`
          (`self.SetActorScale3D` (`KismetMathLibrary.MakeVector` _x_pos _y_pos _z_pos))))
      (else
        (goto _label :!via `Reverse`)))))

(fn `Set Is Pushable`
  (params (`Is pushable` :type Boolean))
  (bind _pushable (`self.Pushable`))
  (if `Is pushable`
    (`/Game/Components/Pushable.Enable push` _pushable)
    (else
      (`/Game/Components/Pushable.Disable push` _pushable))))

(fn `UserConstructionScript`)